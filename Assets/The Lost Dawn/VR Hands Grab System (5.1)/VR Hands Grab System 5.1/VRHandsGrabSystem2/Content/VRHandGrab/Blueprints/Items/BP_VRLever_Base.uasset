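; Base VR lever actor that a player grabs and rotates with a motion controller, showing its position through an indicator light.
; GrabComponent events store the controller and enable Tick only while the lever is held.
; Each tick sets lever pitch from the clamped angle between the base's forward vector and the base-to-hand direction.
; That angle swaps the base's emissive material between red and green, with a small dead band between them.
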(event OnGrabbed(GrabComponent)
  (params (MotionController :type Motion%20Controller%20Component%20Object%20Reference) (GrabType :type E_GrabType%20Enum :default "NewEnumerator2") (GrabComponent :type AC%20Grab%20Component%20Object%20Reference))
  (Variables|Default|SetMCRef MotionController)
  (Variables|Default|SetbIsHeld true)
  (Actor|Tick|SetActorTickEnabled true))

(event OnDropped(GrabComponent)
  (params (GrabType :type E_GrabType%20Enum :default "NewEnumerator2"))
  (Variables|Default|SetMCRef 0)
  (Variables|Default|SetbIsHeld false)
  (Actor|Tick|SetActorTickEnabled false))

(event Custom|RotateLever
  (bind _mcref (Variables|Default|GetMCRef))
  (bind _sm_leverbase (Variables|Default|GetSM_LeverBase))
  (bind _sm_lever (Variables|Default|GetSM_Lever))
  (bind _sm_leverbase_2 (Variables|Default|GetSM_LeverBase))
  (bind _returnvalue (Math|Vector|GetForwardVector _sm_leverbase))
  (bind _returnvalue_2 (Transformation|GetWorldLocation _mcref))
  (bind _returnvalue_3 (Transformation|GetWorldLocation _sm_leverbase))
  (bind _relativerotation (Variables|/Script/Engine.SceneComponent|GetRelativeRotation _sm_lever))
  (bind _returnvalue_4 (- _returnvalue_2 _returnvalue_3))
  (bind _angle (CallFunction|MFGetAngleBtwTwoVectors _returnvalue_4 _returnvalue))
  (bind _returnvalue_5 (- _angle 9e+01))
  (bind _returnvalue_6 (Math|Float|Clamp(Float) _returnvalue_5 -58.0 58.0))
  ;[1 1 1] Rotate lever on tick when grabbed
  (Transformation|SetRelativeRotation _sm_lever (Math|Rotator|MakeRotator (.roll _relativerotation) _returnvalue_6 (.yaw _relativerotation)) false false)
  (Utilities|FlowControl|Sequence
    (:then_0
      (if (< _returnvalue_6 0.0)
        (Rendering|Material|SetMaterial _sm_leverbase_2 1 "/Game/VRHandGrab/Materials/Instances/MI_EmissiveLightRed.MI_EmissiveLightRed")))
    (:then_1
      (if (> _returnvalue_6 1e+01)
        (Rendering|Material|SetMaterial _sm_leverbase_2 1 "/Game/VRHandGrab/Materials/Instances/MI_EmissiveLightGreen.MI_EmissiveLightGreen")))))

(event Custom|FindAngle
  ;[1 1 1] Rotate lever on tick when grabbed
)

(event EventBeginPlay)

(event Collision|EventActorBeginOverlap
  (params (OtherActor :type Actor%20Object%20Reference)))

(event EventTick
  (params (DeltaSeconds :type Float%20%28single-precision%29))
  (if (Variables|Default|GetbIsHeld)
    (CallFunction|RotateLever)))

(fn ConstructionScript)