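; Base VR grenade item that the player grabs, arms by pulling the safety pin, and throws to explode.
; Holding it with the right grab component enables the left one, which breaks the pin's physics constraint and arms the grenade.
; Dropping an armed grenade launches the safety lever with physics impulses and starts a randomized fuse.
; Explosion spawns particles and sound, hides the actor, then destroys it after a delay, without applying damage.
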(event OnGrabbed(GrabComponentRight)
  (params (MotionController :type Motion%20Controller%20Component%20Object%20Reference) (GrabType :type E_GrabType%20Enum :default "NewEnumerator2") (GrabComponent :type AC%20Grab%20Component%20Object%20Reference))
  ;[1 1 1] Events Grab Component Right
  (Variables|Default|SetbIsHeld true)
  ;;[1 1 1] Enable second grab component
  (Variables|/Game/VRHandGrab/Blueprints/ACGrabComponent.ACGrabComponent_C|SetEnabled (Variables|Default|GetGrabComponentLeft) true))

(event OnDropped(GrabComponentRight)
  (params (GrabType :type E_GrabType%20Enum :default "NewEnumerator2"))
  ;[1 1 1] Events Grab Component Right
  ;;[1 1 1] Grenade throw
  (Variables|Default|SetbIsHeld false)
  ;;;[1 1 1] Enable second grab component
  (Variables|/Game/VRHandGrab/Blueprints/ACGrabComponent.ACGrabComponent_C|SetEnabled (Variables|Default|GetGrabComponentLeft) false)
  ;;[1 1 1] If grenade was armed then push lever away
  (if (Variables|Default|GetArmed)
    (CallFunction|PushSafetyLeverAway)))

(event OnGrabbed(GrabComponentLeft)
  (params (MotionController :type Motion%20Controller%20Component%20Object%20Reference) (GrabType :type E_GrabType%20Enum :default "NewEnumerator2") (GrabComponent :type AC%20Grab%20Component%20Object%20Reference))
  ;[1 0.2396 0.2396] Events Grab Component Left remove the safety pin from the grenade and set grenade state to "Armed"
  (Physics|SetSimulatePhysics (Variables|Default|GetSM_Limonka_SafetyPin) false)
  (Class|PhysicsConstraintComponent|BreakConstraint (Variables|Default|GetPhysicsConstraint_0))
  (Variables|Default|SetArmed true))

(event OnDropped(GrabComponentLeft)
  (params (GrabType :type E_GrabType%20Enum :default "NewEnumerator2"))
  ;[1 1 1] On dropped left component (Drop safety pin)
  (Transformation|DetachFromComponent (Variables|Default|GetSM_Limonka_SafetyPin) "KeepWorld" "KeepWorld" "KeepWorld" true)
  (Physics|SetSimulatePhysics (Variables|Default|GetSM_Limonka_SafetyPin) true)
  (Utilities|FlowControl|Delay 0.2)
  (Variables|/Game/VRHandGrab/Blueprints/ACGrabComponent.ACGrabComponent_C|SetEnabled (Variables|Default|GetGrabComponentLeft) false))

(event Custom|PushSafetyLeverAway
  (bind _sm_limonka_safetylever (Variables|Default|GetSM_Limonka_SafetyLever))
  ;[1 0.3194 0] Explosion logic
  ;;[1 1 1] Push safety lever away
  (Physics|SetSimulatePhysics _sm_limonka_safetylever true)
  (Physics|AddImpulse _sm_limonka_safetylever (* (Math|Vector|GetUpVector _sm_limonka_safetylever) 2.5e+02) "None" true)
  (Class|PrimitiveComponent|AddAngularImpulseinDegrees _sm_limonka_safetylever "300.000000,300.000000,300.000000" "None" true)
  (CallFunction|StartFusionTimer))

(event Custom|StartFusionTimer
  ;[1 0.3194 0] Explosion logic
  ;;[1 1 1] Start fusion timer
  (Utilities|FlowControl|Delay (Math|Random|RandomFloatinRange (Variables|Default|GetFusionTimerMin) (Variables|Default|GetFusionTimerMax)))
  (CallFunction|Explosion))

(event Custom|Explosion
  ;[1 0.3194 0] Explosion logic
  ;;[1 1 1] Explosion
  (Development|PrintString "Boom" true false)
  (Effects|SpawnEmitteratLocation "/Game/VRHandGrab/Particles/P_GrenadeExplosion.P_GrenadeExplosion" (Transformation|GetWorldLocation (Variables|Default|GetSM_Item)) "0, 0, 0" "1.300000,1.300000,1.300000")
  (Audio|PlaySoundatLocation "/Game/VRHandGrab/Sound/SC_GrenadeExplosion.SC_GrenadeExplosion" (Transformation|GetActorLocation) "0, 0, 0" 1.0 1.0 0.0 0 0 0 0)
  (Rendering|SetActorHiddenInGame true)
  (Utilities|FlowControl|Delay 3.0)
  (Actor|DestroyActor))

(event EventTriggerReleased
  ;[1 1 1] Events Grab Component Right
)

(event EventTriggerPressed
  ;[1 1 1] Events Grab Component Right
)

(event EventBeginPlay
  (|CallParentFunction))

(event EventTick
  (params (DeltaSeconds :type Float%20%28single-precision%29)))

(fn ConstructionScript
  (|CallParentFunction))