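; Base VR throwable axe that can be grabbed by two grab components and sticks into what it hits, whether held or thrown.
; Above a speed threshold, Tick line-traces from blade arrows, then stops physics and pushes the axe deeper.
; A held hit releases the grab but keeps the hand attached for pulling out.
; Throws can rotate the axe along its velocity, predict the projectile path and snap to the predicted impact rotation when close.
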(event OnGrabbed(GrabComponentRight)
  (params (MotionController :type Motion%20Controller%20Component%20Object%20Reference) (GrabType :type E_GrabType%20Enum :default "NewEnumerator2") (GrabComponent :type AC%20Grab%20Component%20Object%20Reference))
  ;[1 1 1] Grab / Drop for Component Right
  (Variables|Default|SetGrabCompFirstInitiatedGrab GrabComponent)
  (Variables|Default|SetbIsHeld true)
  (Actor|Tick|SetActorTickEnabled true) ; Enable tick when grabbed
  (CallFunction|Reset)
  ;;[1 1 1] Disable hit trace for a moment, so item can be freely grabbed after it hit smth
  (Variables|Logic|SetPenetrationTraceEnabled false)
  (Utilities|FlowControl|RetriggerableDelay 0.2)
  (CallFunction|Reset2)
  (Variables|Logic|SetPenetrationTraceEnabled true))

(event OnDropped(GrabComponentRight)
  (params (GrabType :type E_GrabType%20Enum :default "NewEnumerator2"))
  ;[1 1 1] Grab / Drop for Component Right
  (Variables|Default|SetbIsHeld false)
  (Variables|Logic|SetItemHitSmthDuringPhysSim false)
  (Utilities|FlowControl|Delay 0.1)
  (if (not (CallFunction|CheckifCompGrabbedbyOtherHand))
    (CallFunction|ApplyRotation)))

(event OnGrabbed(GrabComponentLeft)
  (params (MotionController :type Motion%20Controller%20Component%20Object%20Reference) (GrabType :type E_GrabType%20Enum :default "NewEnumerator2") (GrabComponent :type AC%20Grab%20Component%20Object%20Reference))
  ;[1 1 1] Grab / Drop for Component Right
  (Variables|Default|SetGrabCompFirstInitiatedGrab GrabComponent)
  (Variables|Default|SetbIsHeld true)
  (Actor|Tick|SetActorTickEnabled true) ; Enable tick when grabbed
  (CallFunction|Reset)
  ;;[1 1 1] Disable hit trace for a moment, so item can be freely grabbed after it hit smth
  (Variables|Logic|SetPenetrationTraceEnabled false)
  (Utilities|FlowControl|RetriggerableDelay 0.2)
  (CallFunction|Reset2)
  (Variables|Logic|SetPenetrationTraceEnabled true))

(event OnComponentHit(SM_Item)
  (params (HitComponent :type Primitive%20Component%20Object%20Reference) (OtherActor :type Actor%20Object%20Reference) (OtherComp :type Primitive%20Component%20Object%20Reference) (NormalImpulse :type Vector :default "0, 0, 0") (Hit :type Hit%20Result%20Structure%20%28by%20ref%29))
  ;[1 1 1] On Item hit smth
  (if (!= OtherActor self)
    (Variables|Logic|SetItemHitSmthDuringPhysSim true)))

(event OnDropped(GrabComponentLeft)
  (params (GrabType :type E_GrabType%20Enum :default "NewEnumerator2"))
  ;[1 1 1] Grab / Drop for Component Right
  (Variables|Default|SetbIsHeld false)
  (Variables|Logic|SetItemHitSmthDuringPhysSim false)
  (Utilities|FlowControl|Delay 0.1)
  (if (not (CallFunction|CheckifCompGrabbedbyOtherHand))
    (CallFunction|ApplyRotation)))

(event Custom|RotateItemTowardsThrowDirection
  (bind _sm_item (Variables|Default|GetSM_Item))
  ;[1 1 1] On throw -> Rotate item towards throwing direction
  (bind _output_get (Variables|Logic|SetRotationTowardsThrow (Math|Rotator|MakeRotfromX (Transformation|GetComponentVelocity _sm_item))))
  (Transformation|SetWorldRotation _sm_item _output_get false false))

(event Custom|PredictProjectilePath
  ;[1 1 1] Predict path
  (bind _output_get (Variables|Logic|SetThrowStartPos (Transformation|GetWorldLocation (Variables|Default|GetSM_Item))))
  (bind (_outhit _outpathpositions _outlasttracedestination _returnvalue) (Class|GameplayStatics|BlueprintPredictProjectilePathbyTraceChannel _output_get (Transformation|GetComponentVelocity (Variables|Default|GetSM_Item)) true 3.0 "ECC_Visibility" false (Utilities|Array|MakeArray self (Pawn|GetControlledPawn (Game|GetPlayerController 0))) "None" 1e+01))
  (bind _output_get_2 (Variables|Logic|SetPredictedHitBlockSuccessfully _returnvalue))
  (if _output_get_2
    (Variables|Logic|SetPredictedHitLoc (.Location (Collision|BreakHitResult _outhit)))
    (Variables|Logic|SetPredictedRotationOnHit (Math|Rotator|FindLookatRotation (Utilities|Array|Get(acopy) _outpathpositions (- (Utilities|Array|LastIndex _outpathpositions) 1)) (Utilities|Array|Get(acopy) _outpathpositions (Utilities|Array|LastIndex _outpathpositions))))))

(event Custom|ApplyRotation
  ;[1 1 1] Apply rotation
  (if (Math|Boolean|ANDBoolean (Variables|ForDesigner|GetAutoRotateOnceAfterRelease) (Variables|Logic|GetAllowToChangeRot) (> (Variables|Logic|GetCurSpeed) (Variables|ForDesigner|GetApplyTowardsRotationOnceAtSpeed)))
    (CallFunction|RotateItemTowardsThrowDirection)
    (if (Variables|ForDesigner|GetAutCorrectRotationBeforeHit)
      (CallFunction|PredictProjectilePath))))

(event Custom|Reset
  ;[0.03434 0.03434 0.03434] Event Tick
  ;;[1 1 1] Auto Correct Rotation Before Hit
  (Utilities|FlowControl|DoOnce false) ; enters at Reset
)

(event Custom|ItemPenetratedObj)

(event Custom|Reset2
  ;[0.03434 0.03434 0.03434] Event Tick
  ;;[1 0.2396 0.2396] On Line Trace Hit object
  (Utilities|FlowControl|DoOnce false) ; enters at Reset
)

(event EventBeginPlay
  (|CallParentFunction))

(event EventTick
  (params (DeltaSeconds :type Float%20%28single-precision%29))
  (bind _traceoptions (Variables|ForDesigner|GetTraceOptions))
  (bind (_middletrace _lefttrace _righttrace) (Utilities|Struct|BreakS_TraceOptions _traceoptions))
  ;[0.03434 0.03434 0.03434] Event Tick
  (|CallParentFunction DeltaSeconds)
  (Utilities|FlowControl|Sequence
    (:then_0
      ;;[1 0.2396 0.2396] On Line Trace Hit object
      (if (> (Variables|Logic|GetCurSpeed) (Variables|ForDesigner|GetPenetrateIfSpeedGreaterThan))
        (bind (_outhit _returnvalue) (CallFunction|HitTracefromArrow "None" (Variables|ForDesigner|GetHitTracelength) _middletrace _lefttrace _righttrace))
        (Variables|Logic|SetOut%20Hit _outhit)
        (if (Variables|Default|GetbIsHeld)
          (if (and _returnvalue (Variables|Logic|GetPenetrationTraceEnabled))
            (Utilities|FlowControl|DoOnce false :!label _label
              (:Completed
                (Variables|Logic|SetSpeedWhenSmthWasHit (Variables|Logic|GetCurSpeed))
                (Variables|Logic|SetItemHitSmthDuringPhysSim true)
                (if (Variables|Default|GetbIsHeld)
                  ;;;[0 1 0.5686] Hit when held in hand
                  (Variables|Logic|SetAllowToChangeRot false)
                  (Default|TryRelease (Variables|Default|GetGrabCompFirstInitiatedGrab) false) ; Release grabbed item for penetration effect. And do not clear attached actor ref, so that hand will be still attached to the item
                  (Physics|SetSimulatePhysics (Variables|Default|GetSM_Item) false)
                  ;;;;[1 0.776 0.1602] Add extra penetration for item in forward direction
                  (CallFunction|AddExtraPenetrationinForwardDir (+ (.Distance (Collision|BreakHitResult (Variables|Logic|GetOut%20Hit))) (Variables|ForDesigner|GetAddExtraPenetrationOnHit)))
                  (Default|BindEventtoDispatcher (Variables|Default|GetGrabCompFirstInitiatedGrab) (Math|Vector|GetForwardVector (Variables|Default|GetArrowMiddlePenetration))) ; Grab again after penetration if user pulls item in opposite direction of the hit
                  (else
                    ;;;[0 1 0.5686] Hit when Thrown
                    (Physics|SetSimulatePhysics (Variables|Default|GetSM_Item) false) ; Stop simulating if item was thrown
                    ;;;;[1 0.776 0.1602] Add extra penetration for item in forward direction
                    (CallFunction|AddExtraPenetrationinForwardDir (+ (.Distance (Collision|BreakHitResult (Variables|Logic|GetOut%20Hit))) (Variables|ForDesigner|GetAddExtraPenetrationOnHit)))
                    (Variables|Logic|SetPredictedHitBlockSuccessfully false))))))
          (elif (and _returnvalue (Variables|Logic|GetPenetrationTraceEnabled))
            (goto _label)))))
    (:then_1
      ;;[1 1 1] Auto Correct Rotation Before Hit
      (if (Math|Boolean|ANDBoolean (Variables|Logic|GetPredictedHitBlockSuccessfully) (not (Variables|Logic|GetItemHitSmthDuringPhysSim)) (Variables|ForDesigner|GetAutCorrectRotationBeforeHit) (not (Variables|Default|GetbIsHeld)) (Variables|Logic|GetAllowToChangeRot) (> (Variables|Logic|GetCurSpeed) 2.0)) ; Make Rotation Correction if was made prediction and object didn't hit smth already
        (if (< (Math|Vector|Distance(Vector) (Transformation|GetWorldLocation (Variables|Default|GetSM_Item)) (Variables|Logic|GetPredictedHitLoc)) (Variables|ForDesigner|GetCorrectionRangeKickIn))
          (Utilities|FlowControl|Sequence
            (:then_0
              (Utilities|FlowControl|DoOnce false
                (:Completed
                  (Variables|Logic|SetTransformBeforeAutoCorrKickedIn (Transformation|GetWorldTransform (Variables|Default|GetSM_Item))))))
            (:then_1
              (Transformation|SetWorldRotation (Variables|Default|GetSM_Item) (Variables|Logic|GetPredictedRotationOnHit) false false))))))
    (:then_2
      (Variables|Logic|SetCurSpeed (CallFunction|GetItemSpeedonTick)))))

(fn ConstructionScript
  (|CallParentFunction))

(fn HitTracefromArrow
  (params (DrawDebugType :type EDrawDebugTrace%20Enum :default "None") (Tracelength :type Float%20%28double-precision%29) (MiddleTrace :type Boolean) (LeftTrace :type Boolean) (RightTrace :type Boolean))
  (for (_array_element _array_index) (Utilities|Array|MakeArray (Variables|Default|GetArrowMiddlePenetration) (Variables|Default|GetArrowLeftPenetration) (Variables|Default|GetArrowRightPenetration))
    (if (Utilities|Select :Index _array_index :Option%200 MiddleTrace :Option%201 LeftTrace :Option%202 RightTrace)
      (bind (_outhit _returnvalue) (Collision|LineTraceByChannel (Transformation|GetWorldLocation _array_element) (+ (Transformation|GetWorldLocation _array_element) (* (Math|Vector|GetForwardVector _array_element) Tracelength)) "TraceTypeQuery1" false 0 DrawDebugType))
      (if _returnvalue
        (LocalVariables|SetHitBlock _returnvalue)
        (LocalVariables|SetHit _outhit))))
  (return (LocalVariables|GetHit) (LocalVariables|GetHitBlock)))

(fn GetItemSpeedonTick
  (bind _sm_item (Variables|Default|GetSM_Item))
  (bind _returnvalue (Transformation|GetWorldLocation _sm_item))
  (LocalVariables|SetItemSpeed (Math|Vector|Distance(Vector) _returnvalue (Variables|Logic|GetOldLoc)))
  (Variables|Logic|SetOldLoc _returnvalue)
  (return (LocalVariables|GetItemSpeed)))

(fn CheckifCompGrabbedbyOtherHand
  (for _array_element (Actor|GetComponentsByClass "/Game/VRHandGrab/Blueprints/ACGrabComponent.ACGrabComponent_C")
    (if (Variables|/Game/VRHandGrab/Blueprints/ACGrabComponent.ACGrabComponent_C|GetbIsHeld _array_element)
      (Variables|Default|SetGrabbedByOtherHand (Variables|/Game/VRHandGrab/Blueprints/ACGrabComponent.ACGrabComponent_C|GetbIsHeld _array_element))))
  (return (Variables|Default|GetGrabbedByOtherHand)))

(fn AddExtraPenetrationinForwardDir
  (params (AddValue :type Float%20%28double-precision%29))
  ;[1 1 1] Add extra penetration for item in forward direction
  (bind _output_get (LocalVariables|SetNewLoc (+ (Transformation|GetWorldLocation (Variables|Default|GetSM_Item)) (* (Math|Vector|GetForwardVector (Variables|Default|GetArrowMiddlePenetration)) AddValue))))
  (Transformation|SetWorldLocation (Variables|Default|GetSM_Item) _output_get false false)
  (return (LocalVariables|GetNewLoc)))

(fn GetGrabCompWhichIsAttachedtoMC
  (for _array_element (Actor|GetComponentsByClass "/Game/VRHandGrab/Blueprints/ACGrabComponent.ACGrabComponent_C")
    (if (Variables|/Game/VRHandGrab/Blueprints/ACGrabComponent.ACGrabComponent_C|GetbIsHeld _array_element)
      (LocalVariables|SetGrabCompLocal _array_element)))
  (return (LocalVariables|GetGrabCompLocal)))